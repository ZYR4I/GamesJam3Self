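; Parent Blueprint for melee enemies that detect the player, attack, take damage and die.
; A sphere overlap by the player pawn notifies the AI controller, and Attack plays a random montage.
; CheckHit sphere-traces at a given bone to damage the player character.
; Incoming damage updates a health bar widget; at zero health, a random death montage plays while AI logic and collision stop, and the actor is destroyed on blend out.
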(event `self.ReceiveBeginPlay`
  (bind _maxhealth (`self.MaxHealth`))
  (bind _asbp_ai_controller (cast `/Game/Blueprints/Enemies/BP_AiController` (`self.GetController`)))
  (set `self.ControllerRef` _asbp_ai_controller)
  (bind _output_get (set `self.CurrentHealth` _maxhealth))
  (bind _aswbp_health_bar (cast `/Game/Blueprints/HUD/WBP_HealthBar` (`WidgetComponent.GetUserWidgetObject` (`self.HealthBar`))))
  (bind _output_get_2 (set `self.WidgetRef` _aswbp_health_bar))
  (set `/Game/Blueprints/HUD/WBP_HealthBar.%Health` (/ _output_get _maxhealth) _output_get_2))

(event `self.Sphere.OnComponentBeginOverlap`
  (params (OverlappedComponent :type "PrimitiveComponent Object Reference") (OtherActor :type "Actor Object Reference") (OtherComp :type "PrimitiveComponent Object Reference") (OtherBodyIndex :type Integer) (bFromSweep :type Boolean) (SweepResult :type "HitResult Structure (by ref)"))
  ;[1 1 1] PlayerOverlapped
  (if (== OtherActor (`GameplayStatics.GetPlayerPawn` 0))
    (`/Game/Blueprints/Enemies/BP_AiController.PlayerSeen` (`self.ControllerRef`))))

(event `Attack`
  ;[1 1 1] Attack Anim
  (`|PlayMontage` (`self.Mesh`) (`KismetArrayLibrary.Array_Random` (`self.AttackAnimations`))))

(event `CheckHit`
  (params (BoneName :type Name))
  (bind _returnvalue (`SceneComponent.GetSocketLocation` (`self.Mesh`) BoneName))
  ;[1 1 1] CheckHit
  (bind _outhit (`KismetSystemLibrary.SphereTraceSingle` _returnvalue _returnvalue 200.0 "TraceTypeQuery2" false (`self.GetAllChildActors` self true)))
  (bind _asbp_player_character_parent (cast `/Game/Blueprints/Player/BP_PlayerCharacterParent` (`.HitActor` (`GameplayStatics.BreakHitResult` _outhit))))
  (`GameplayStatics.ApplyDamage` _asbp_player_character_parent (`self.Damage`) null self))

(event `self.ReceiveAnyDamage`
  (params (Damage :type "Float (single-precision)") (DamageType :type "DamageType Object Reference") (InstigatedBy :type "Controller Object Reference") (DamageCauser :type "Actor Object Reference"))
  ;[1 1 1] Damaged
  (bind _output_get (set `self.CurrentHealth` (- (`self.CurrentHealth`) Damage)))
  (`self.UpdateHealthBar`)
  (if (<= _output_get 0.0)
    (`|PlayMontage` (`self.Mesh`) (`KismetArrayLibrary.Array_Random` (`self.DeathAnims`))
      (:`then`
        (`self.Death`))
      (:`OnBlendOut`
        (`self.K2_DestroyActor`)))))

(fn `UpdateHealthBar`
  (set `/Game/Blueprints/HUD/WBP_HealthBar.%Health` (/ (`self.CurrentHealth`) (`self.MaxHealth`)) (`self.WidgetRef`)))

(fn `UserConstructionScript`)