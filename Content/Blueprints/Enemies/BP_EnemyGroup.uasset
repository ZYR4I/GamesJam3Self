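; BP_EnemyGroup is a placeable group of melee enemies that aggro together when the player approaches.
; On BeginPlay it spawns melee imps at its four scene-component points, capped by a DoN on Max, plus an optional double-scale mini boss at BossSpawn.
; It tracks the spawned enemies, and when the player pawn overlaps its sphere, it calls GroupAgroed on each one still valid.
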(event `self.ReceiveBeginPlay`
  (bind _allscenecomponents (`self.AllSceneComponents`))
  (`KismetArrayLibrary.Array_Add` _allscenecomponents (`self.Scene`))
  (`KismetArrayLibrary.Array_Add` _allscenecomponents (`self.Scene1`))
  (`KismetArrayLibrary.Array_Add` _allscenecomponents (`self.Scene2`))
  (`KismetArrayLibrary.Array_Add` _allscenecomponents (`self.Scene3`))
  (for _array_element (`self.AllSceneComponents`)
    (`/Engine/EditorBlueprintResources/StandardMacros.Do N` (`self.Max`)
      (:`Exit`
        (bind _returnvalue (`|SpawnActorFromClass` "/Game/Blueprints/Enemies/BP_MeleeImp.BP_MeleeImp_C" (`KismetMathLibrary.Conv_VectorToTransform` (`SceneComponent.K2_GetComponentLocation` _array_element)) "Undefined" "OverrideRootScale" null null))
        (`KismetArrayLibrary.Array_Add` (`self.SpawnedEnemies`) _returnvalue))))
  (if (`self.SpawnBoss`)
    (bind _returnvalue_2 (`|SpawnActorFromClass` "/Game/Blueprints/Enemies/BP_MeleeEnemyMiniBoss.BP_MeleeEnemyMiniBoss_C" (`KismetMathLibrary.MakeTransform` (`SceneComponent.K2_GetComponentLocation` (`self.BossSpawn`)) (struct) (2.0 2.0 2.0)) "Undefined" "OverrideRootScale" null null))
    (`KismetArrayLibrary.Array_Add` (`self.SpawnedEnemies`) _returnvalue_2)))

(event `self.Sphere.OnComponentBeginOverlap`
  (params (OverlappedComponent :type "PrimitiveComponent Object Reference") (OtherActor :type "Actor Object Reference") (OtherComp :type "PrimitiveComponent Object Reference") (OtherBodyIndex :type Integer) (bFromSweep :type Boolean) (SweepResult :type "HitResult Structure (by ref)"))
  (if (== OtherActor (`GameplayStatics.GetPlayerPawn` 0))
    (for _array_element (`self.SpawnedEnemies`)
      (`/Engine/EditorBlueprintResources/StandardMacros.IsValid` _array_element
        (:`Is Valid`
          (`/Game/Blueprints/Enemies/BP_MeleeEnemyParent.GroupAgroed` _array_element))))))

(fn `UserConstructionScript`)