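; Ranged caster enemy Blueprint that attacks the player with fireballs.
; Its Fireball event spawns a BP_FireBall at the mesh's RightHand socket, rotated toward the first player's current location, and passes in the caster's Damage value.
; The event has no caller within this Blueprint, and the default BeginPlay, overlap and Tick events are unused.
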(event `Fireball`
  (bind _returnvalue (`SceneComponent.GetSocketLocation` (`self.Mesh`) "RightHand"))
  (`|SpawnActorFromClass` "/Game/Blueprints/Enemies/BP_FireBall.BP_FireBall_C" (`KismetMathLibrary.MakeTransform` _returnvalue (`KismetMathLibrary.FindLookAtRotation` _returnvalue (`self.K2_GetActorLocation` (`GameplayStatics.GetPlayerPawn` 0)))) "Undefined" "OverrideRootScale" null (`self.Damage`) null))

(fn `UserConstructionScript`
  (`parent.UserConstructionScript`))