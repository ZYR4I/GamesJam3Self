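; BP_EnemyBoss is an encounter spawner that creates a melee boss enemy and aggroes it when the player gets close.
; On BeginPlay, if SpawnBoss is set, it spawns a double-scale BP_MeleeEnemyBoss at the BossSpawn component and stores it in SpawnedEnemies.
; When the player pawn overlaps the Sphere, it calls GroupAgroed on every stored enemy.
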(event `self.ReceiveBeginPlay`
  (if (`self.SpawnBoss`)
    (bind _returnvalue (`|SpawnActorFromClass` "/Game/Blueprints/Enemies/BP_MeleeEnemyBoss.BP_MeleeEnemyBoss_C" (`KismetMathLibrary.MakeTransform` (`SceneComponent.K2_GetComponentLocation` (`self.BossSpawn`)) (struct) (2.0 2.0 2.0)) "Undefined" "OverrideRootScale" null null))
    (`KismetArrayLibrary.Array_Add` (`self.SpawnedEnemies`) _returnvalue)))

(event `self.Sphere.OnComponentBeginOverlap`
  (params (OverlappedComponent :type "PrimitiveComponent Object Reference") (OtherActor :type "Actor Object Reference") (OtherComp :type "PrimitiveComponent Object Reference") (OtherBodyIndex :type Integer) (bFromSweep :type Boolean) (SweepResult :type "HitResult Structure (by ref)"))
  (if (== OtherActor (`GameplayStatics.GetPlayerPawn` 0))
    (for _array_element (`self.SpawnedEnemies`)
      (`/Game/Blueprints/Enemies/BP_MeleeEnemyParent.GroupAgroed` _array_element))))

(fn `UserConstructionScript`)