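; BP_FireBall is an enemy fireball projectile that homes in on the player and deals damage on contact.
; On BeginPlay it sets the player pawn's root component as the ProjectileMovement homing target.
; When Sphere1 overlaps the capsule component of a BP_CharacterParent, it applies Damage once to that actor and destroys itself.
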(event `self.ReceiveBeginPlay`
  (set `ProjectileMovementComponent.HomingTargetComponent` (`Actor.RootComponent` (`GameplayStatics.GetPlayerPawn` 0)) (`self.ProjectileMovement`)))

(event `self.Sphere1.OnComponentBeginOverlap`
  (params (OverlappedComponent :type "PrimitiveComponent Object Reference") (OtherActor :type "Actor Object Reference") (OtherComp :type "PrimitiveComponent Object Reference") (OtherBodyIndex :type Integer) (bFromSweep :type Boolean) (SweepResult :type "HitResult Structure (by ref)"))
  (bind _asbp_character_parent (cast `/Game/Blueprints/Player/Player/BP_CharacterParent` OtherActor))
  (if (== (`Character.CapsuleComponent` _asbp_character_parent) OtherComp)
    (`/Engine/EditorBlueprintResources/StandardMacros.DoOnce` false
      (:`Completed`
        (`GameplayStatics.ApplyDamage` OtherActor (`self.Damage`))
        (`self.K2_DestroyActor`)))))

(fn `UserConstructionScript`)