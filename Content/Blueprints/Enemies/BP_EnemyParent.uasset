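; Base enemy character that chases and attacks the player, takes damage and pays out reward money on death.
; It feeds group aggro, attack-range overlaps and attack completion to BP_AiController, playing random attack montages and applying damage when its hitbox overlaps the player.
; Damage updates a widget health bar and spawns floating numbers; death stops AI logic and collision, then destroys the actor after a death montage.
; A timed slow temporarily reduces walk speed.
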(event `self.ReceiveBeginPlay`
  (bind _maxhealth (`self.MaxHealth`))
  (bind _asbp_ai_controller (cast `/Game/Blueprints/Enemies/BP_AiController` (`self.GetController`)))
  (set `self.ControllerRef` _asbp_ai_controller)
  (bind _output_get (set `self.CurrentHealth` _maxhealth))
  (bind _aswbp_health_bar (cast `/Game/Blueprints/HUD/WBP_HealthBar` (`WidgetComponent.GetUserWidgetObject` (`self.HealthBar`))))
  (bind _output_get_2 (set `self.WidgetRef` _aswbp_health_bar))
  (set `/Game/Blueprints/HUD/WBP_HealthBar.%Health` (/ _output_get _maxhealth) _output_get_2)
  (set `self.DefaultSpeed` (`CharacterMovementComponent.MaxWalkSpeed` (`self.CharacterMovement`)))
  (`/Game/Blueprints/Enemies/BP_AiController.SetAttackRange` (`self.ControllerRef`) (/ (`SphereComponent.GetScaledSphereRadius` (`self.AttackRange`)) 2.0)))

(event `GroupAgroed`
  ;[1 1 1] Aggro
  (`/Game/Blueprints/Enemies/BP_AiController.PlayerSeen` (`self.ControllerRef`))
  (`AIController.K2_SetFocus` (`self.ControllerRef`) (`GameplayStatics.GetPlayerPawn` 0)))

(event `AttackAnim`
  (bind (_returnvalue_roll _returnvalue_pitch _returnvalue_yaw) (`KismetMathLibrary.BreakRotator` (`KismetMathLibrary.FindLookAtRotation` (`self.K2_GetActorLocation`) (`self.K2_GetActorLocation` (`GameplayStatics.GetPlayerPawn` 0)))))
  ;[1 1 1] Attack Anim
  (`KismetSystemLibrary.PrintString` "Hello")
  (`|PlayMontage` (`self.Mesh`) (`KismetArrayLibrary.Array_Random` (`self.AttackAnimations`))
    (:`then`
      _)
    (:`OnBlendOut`
      _))
  (`self.K2_SetActorRotation` (`KismetMathLibrary.MakeRotator` 0.0 0.0 _returnvalue_yaw))
  (`/Game/Blueprints/Enemies/BP_AiController.Attacked` (`self.ControllerRef`) (`self.AttackSpeed`)))

(event `CheckHit`
  (params (BoneName :type Name))
  (bind _overlappingactors (`PrimitiveComponent.GetOverlappingActors` (`self.HitBox`) "/Game/Blueprints/Player/Player/BP_CharacterParent.BP_CharacterParent_C"))
  ;[1 1 1] CheckHit
  (bind _asbp_character_parent (cast `/Game/Blueprints/Player/Player/BP_CharacterParent` (`|GetArrayItem` _overlappingactors (`KismetArrayLibrary.Array_Find` _overlappingactors (`GameplayStatics.GetPlayerPawn` 0)))))
  (`GameplayStatics.ApplyDamage` _asbp_character_parent (`self.Damage`) null self))

(event `self.ReceiveAnyDamage`
  (params (Damage :type "Float (single-precision)") (DamageType :type "DamageType Object Reference") (InstigatedBy :type "Controller Object Reference") (DamageCauser :type "Actor Object Reference"))
  ;[1 1 1] Damaged
  (bind _output_get (set `self.CurrentHealth` (- (`self.CurrentHealth`) Damage)))
  (`self.UpdateHealthBar`)
  (if (<= _output_get 0.0)
    (`/Engine/EditorBlueprintResources/StandardMacros.DoOnce` false
      (:`Completed`
        (`|PlayMontage` (`self.Mesh`) (`KismetArrayLibrary.Array_Random` (`self.DeathAnims`))
          (:`then`
            (`self.Death`)
            (`self.DamageNumbers` Damage :!label _label))
          (:`OnBlendOut`
            (`self.K2_DestroyActor`)))))
    (else
      (goto _label))))

(event `Slowed`
  (params (SlowAmmount :type "Float (double-precision)") (SlowTime :type "Float (double-precision)"))
  (bind _charactermovement (`self.CharacterMovement`))
  (bind _defaultspeed (`self.DefaultSpeed`))
  ;[1 1 1] Slowed
  (set `CharacterMovementComponent.MaxWalkSpeed` (- _defaultspeed (* SlowAmmount (/ _defaultspeed 100.0))) _charactermovement)
  (`KismetSystemLibrary.Delay` SlowTime)
  (set `CharacterMovementComponent.MaxWalkSpeed` (`self.DefaultSpeed`) _charactermovement))

(event `self.AttackRange.OnComponentBeginOverlap`
  (params (OverlappedComponent :type "PrimitiveComponent Object Reference") (OtherActor :type "Actor Object Reference") (OtherComp :type "PrimitiveComponent Object Reference") (OtherBodyIndex :type Integer) (bFromSweep :type Boolean) (SweepResult :type "HitResult Structure (by ref)"))
  (cast `/Game/Blueprints/Player/Player/BP_CharacterParent` OtherActor)
  (`/Game/Blueprints/Enemies/BP_AiController.InAttackRange` (`self.ControllerRef`)))

(event `self.AttackRange.OnComponentEndOverlap`
  (params (OverlappedComponent :type "PrimitiveComponent Object Reference") (OtherActor :type "Actor Object Reference") (OtherComp :type "PrimitiveComponent Object Reference") (OtherBodyIndex :type Integer))
  (cast `/Game/Blueprints/Player/Player/BP_CharacterParent` OtherActor)
  (`/Game/Blueprints/Enemies/BP_AiController.LeftAttackRange` (`self.ControllerRef`)))

(fn `UpdateHealthBar`
  (set `/Game/Blueprints/HUD/WBP_HealthBar.%Health` (/ (`self.CurrentHealth`) (`self.MaxHealth`)) (`self.WidgetRef`)))

(fn `UserConstructionScript`)