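; BP_PlayerController is the player controller that turns player input into commands for the controlled pawn.
; Each axis and action event calls a message on that pawn, covering movement, jumping, camera look, attack, shop, pause, two abilities and right-mouse ability cancel.
; Movement messages carry the pawn's forward or right vector, and abilities forward both press and release.
; The messages are interface-style calls without casts, so pawns supply the actual behaviour.
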(event `InputAxis|MoveForward`
  (params (AxisValue :type "Float (single-precision)"))
  (bind _returnvalue (`self.K2_GetPawn`))
  ;[1 1 1] Movement
  (message `/Game/Blueprints/Player/BPI_PlayerInterface.MoveForward` _returnvalue AxisValue (`self.GetActorForwardVector` _returnvalue)))

(event `InputAction|Jump`
  (params (Key :type "Key Structure"))
  (bind _returnvalue (`self.K2_GetPawn`))
  ;[1 1 1] Movement
  (:`Pressed`
    (message `/Game/Blueprints/Player/BPI_PlayerInterface.IJump` _returnvalue))
  (:`Released`
    (message `/Game/Blueprints/Player/BPI_PlayerInterface.IStopJumping` _returnvalue)))

(event `InputAxis|MoveRight`
  (params (AxisValue :type "Float (single-precision)"))
  (bind _returnvalue (`self.K2_GetPawn`))
  ;[1 1 1] Movement
  (message `/Game/Blueprints/Player/BPI_PlayerInterface.MoveRight` _returnvalue AxisValue (`self.GetActorRightVector` _returnvalue)))

(event `InputAxis|MouseX`
  (params (AxisValue :type "Float (single-precision)"))
  ;[1 1 1] CameraMovement
  (message `/Game/Blueprints/Player/BPI_PlayerInterface.LookRight` (`self.K2_GetPawn`) AxisValue))

(event `InputAction|Attack`
  (params (Key :type "Key Structure"))
  ;[1 1 1] Attack
  (:`Pressed`
    (message `/Game/Blueprints/Player/BPI_PlayerInterface.Attack` (`self.K2_GetPawn`))))

(event `InputAxis|MouseY`
  (params (AxisValue :type "Float (single-precision)"))
  ;[1 1 1] CameraMovement
  (message `/Game/Blueprints/Player/BPI_PlayerInterface.LookUp` (`self.K2_GetPawn`) AxisValue))

(event `InputAction|Shop`
  (params (Key :type "Key Structure"))
  ;[1 1 1] Shop
  (:`Pressed`
    (message `/Game/Blueprints/Player/BPI_PlayerInterface.OpenShop` (`self.K2_GetPawn`))))

(event `InputAction|Pause` :paused true
  (params (Key :type "Key Structure"))
  ;[1 1 1] Pause
  (:`Pressed`
    (message `/Game/Blueprints/Player/BPI_PlayerInterface.Pause` (`self.K2_GetPawn`))))

(event `InputAction|Abilty1`
  (params (Key :type "Key Structure"))
  (bind _returnvalue (`self.K2_GetPawn`))
  ;[1 1 1] Ability 1
  (:`Pressed`
    (message `/Game/Blueprints/Player/BPI_PlayerInterface.A1-Pressed` _returnvalue))
  (:`Released`
    (message `/Game/Blueprints/Player/BPI_PlayerInterface.A1-Released` _returnvalue)))

(event `InputAction|Abilty2`
  (params (Key :type "Key Structure"))
  (bind _returnvalue (`self.K2_GetPawn`))
  ;[1 1 1] Ability 2
  (:`Pressed`
    (message `/Game/Blueprints/Player/BPI_PlayerInterface.A2-Pressed` _returnvalue))
  (:`Released`
    (message `/Game/Blueprints/Player/BPI_PlayerInterface.A2-Released` _returnvalue)))

(event `InputAction|CancelAbility`
  (params (Key :type "Key Structure"))
  (bind _returnvalue (`self.K2_GetPawn`))
  ;[1 1 1] RightMouseButton
  (:`Pressed`
    (message `/Game/Blueprints/Player/BPI_PlayerInterface.RMB-Held` _returnvalue))
  (:`Released`
    (message `/Game/Blueprints/Player/BPI_PlayerInterface.RMB_Released` _returnvalue)))

(fn `UserConstructionScript`)