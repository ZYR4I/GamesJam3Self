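; Melee player character with a held-click three-hit combo and two mana-costed, cooldown-gated abilities.
; Montage blend-outs chain attacks; CheckHit damages the closest target, or cleaves all in range at half damage on the third swing, with lifesteal.
; Abilities preview while held, cancel on RMB and play montages on release.
; Ability1 box-traces a forward line; Ability2 sphere-traces around the player, knocking enemies back, and both update widget cooldowns.
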(event `/Game/Blueprints/Player/BPI_PlayerInterface.Attack`
  (bind _mesh (`self.Mesh`))
  (bind _stat_attackspeed (`self.Stat_AttackSpeed`))
  (bind _returnvalue (`PlayerController.IsInputKeyDown` (`GameplayStatics.GetPlayerController` 0) "LeftMouseButton"))
  ;[1 1 1] Attack Sequence
  (`/Engine/EditorBlueprintResources/StandardMacros.DoOnce` false :!label _label
    (:`Completed`
      (set `self.IsAttacking` true)
      (`|PlayMontage` _mesh "/Game/Blueprints/Player/Melee_Mesh/AttackAnimations/AM_Attack1.AM_Attack1" _stat_attackspeed :!label _label_2
        (:`then`
          (set `self.AttackEnum` "NewEnumerator0"))
        (:`OnCompleted`
          (`self.ComboReset` :!label _label_3))
        (:`OnBlendOut`
          (if _returnvalue
            (`|PlayMontage` _mesh "/Game/Blueprints/Player/Melee_Mesh/AttackAnimations/AM_Attack2.AM_Attack2" _stat_attackspeed
              (:`OnCompleted`
                (goto _label_3))
              (:`OnBlendOut`
                (if _returnvalue
                  (`|PlayMontage` _mesh "/Game/Blueprints/Player/Melee_Mesh/AttackAnimations/AM_Attack3.AM_Attack3" _stat_attackspeed
                    (:`then`
                      (set `self.AttackEnum` "NewEnumerator1"))
                    (:`OnCompleted`
                      (goto _label_3))
                    (:`OnBlendOut`
                      (if _returnvalue
                        (goto _label_2)))))))))))))

(event `self.ComboReset`
  ;[1 1 1] Attack Sequence
  (set `self.IsAttacking` false)
  (goto _label :!via `Reset`))

(event `self.CheckHit`
  (params (BoneName :type Name))
  (bind _targetsinrange (`self.TargetsInRange`))
  ;[1 1 1] CheckHit
  (switch `/Game/Blueprints/Player/Enum_AttackEnum` (`self.AttackEnum`)
    (:`NewEnumerator0`
      (bind _closest (`self.F_FindClosestTarget` (`self.TargetsInRange`) :!label _label_4))
      (bind _returnvalue (`GameplayStatics.ApplyDamage` _closest (`self.Stat_PlayerDamage`) null self))
      (`self.F_LifeSteal` _returnvalue))
    (:`NewEnumerator1`
      (if (< (`KismetArrayLibrary.Array_Length` _targetsinrange) 2)
        (goto _label_4)
        (else
          (for _array_element _targetsinrange
            (bind _returnvalue_2 (`GameplayStatics.ApplyDamage` _array_element (/ (`self.Stat_PlayerDamage`) 2.0) null self))
            (`self.F_LifeSteal` _returnvalue_2)))))))

(event `self.Death`
  ;[1 1 1] Damaged
  (`/Engine/EditorBlueprintResources/StandardMacros.DoOnce` false
    (:`Completed`
      (`|PlayMontage` (`self.Mesh`) "/Game/Blueprints/Player/Melee_Mesh/AM_Death.AM_Death"
        (:`then`
          (`parent.Death`))))))

(event `/Game/Blueprints/Player/BPI_PlayerInterface.RMB-Held`
  (set `self.RMB_Held?` true)
  (`SceneComponent.SetVisibility` (`self.Ability1Display`) false false)
  (`SceneComponent.SetVisibility` (`self.Ability2Display`) false false))

(event `/Game/Blueprints/Player/BPI_PlayerInterface.A1-Pressed`
  ;[1 1 1] Ability 1
  ;;[1 1 1] AbilityButtonPressed
  (if (not (`self.A1OnCooldown`))
    (bind _cancast (`self.F_ManaCheck` 1))
    (if _cancast
      (`SceneComponent.SetVisibility` (`self.Ability1Display`) true false)
      (set `self.RMB_Held?` false))))

(event `/Game/Blueprints/Player/BPI_PlayerInterface.A1-Released`
  (bind _returnvalue (`GameplayStatics.GetPlayerController` 0))
  ;[1 1 1] Ability 1
  ;;[1 1 1] AbilityButtonPressed
  (if (`self.RMB_Held?`)
    _
    (elif (`SceneComponent.bVisible` (`self.Ability1Display`))
      (`SceneComponent.SetVisibility` (`self.Ability1Display`) false false)
      (`|PlayMontage` (`self.Mesh`) "/Game/Blueprints/Player/Melee_Mesh/AbilityAnims/AM_LineAttack.AM_LineAttack"
        (:`then`
          (`self.DisableInput` _returnvalue _returnvalue)
          (`self.ComboReset`)
          (set `self.Stat_CurrentMana` (- (`self.Stat_CurrentMana`) (`self.Ability1ManaCost`)))
          (`self.F_UpdateHealthAndMana` false))))))

(event `self.Ability1`
  (bind _returnvalue (`GameplayStatics.GetPlayerController` 0))
  (bind _returnvalue_2 (`self.K2_GetActorLocation`))
  (bind _returnvalue_3 (`self.K2_GetActorLocation`))
  ;[1 1 1] Ability 1
  ;;[1 1 1] DealAbilityDamage
  (`|ExecutionSequence`
    (:`then_0`
      (bind _outhits (`KismetSystemLibrary.BoxTraceMulti` _returnvalue_2 (+ _returnvalue_2 (* (`self.GetActorForwardVector`) 500.0)) (50.0 50.0 50.0) (struct) "TraceTypeQuery1"))
      (`NiagaraFunctionLibrary.SpawnSystemAtLocation` "/Game/Blueprints/Player/Abilities/FX_Ability1.FX_Ability1" _returnvalue_3 (`KismetMathLibrary.FindLookAtRotation` _returnvalue_3 (+ _returnvalue_3 (`self.GetActorForwardVector`))))
      (for _array_element _outhits
        (bind _asbp_melee_enemy_parent (cast `/Game/Blueprints/Enemies/BP_EnemyParent` (`.HitActor` (`GameplayStatics.BreakHitResult` _array_element))))
        (bind _damageoutput (`self.F_AbilityDamageSet` 1))
        (`GameplayStatics.ApplyDamage` _asbp_melee_enemy_parent _damageoutput null self))
      (`/Game/Blueprints/HUD/WBP_MainHud.Ability1Used` (`self.MainWidgetRef`) (`KismetMathLibrary.FTrunc` (`self.Ability1Cooldown`))))
    (:`then_1`
      (`KismetSystemLibrary.Delay` 0.2)
      (`self.EnableInput` _returnvalue _returnvalue)
      (set `self.A1OnCooldown` true)
      (`KismetSystemLibrary.Delay` (`self.Ability1Cooldown`))
      (set `self.A1OnCooldown` false))))

(event `/Game/Blueprints/Player/BPI_PlayerInterface.A2-Pressed`
  ;[1 1 1] Ability2
  ;;[1 1 1] AbilityButtonPressed
  (if (not (`self.A2OnCooldown`))
    (bind _cancast (`self.F_ManaCheck` 2))
    (if _cancast
      (`SceneComponent.SetVisibility` (`self.Ability2Display`) true false)
      (set `self.RMB_Held?` false))))

(event `/Game/Blueprints/Player/BPI_PlayerInterface.A2-Released`
  (bind _returnvalue (`GameplayStatics.GetPlayerController` 0))
  ;[1 1 1] Ability2
  ;;[1 1 1] AbilityButtonPressed
  (if (`self.RMB_Held?`)
    _
    (elif (`SceneComponent.bVisible` (`self.Ability2Display`))
      (`SceneComponent.SetVisibility` (`self.Ability2Display`) false false)
      (`|PlayMontage` (`self.Mesh`) "/Game/Blueprints/Player/Melee_Mesh/AbilityAnims/AM_Spin.AM_Spin"
        (:`then`
          (`self.DisableInput` _returnvalue _returnvalue)
          (`self.ComboReset`)
          (set `self.Stat_CurrentMana` (- (`self.Stat_CurrentMana`) (`self.Ability2ManaCost`)))
          (`self.F_UpdateHealthAndMana` false))
        (:`OnBlendOut`
          (`self.EnableInput` _returnvalue _returnvalue)
          (set `self.A2OnCooldown` true)
          (`KismetSystemLibrary.Delay` (`self.Ability2Cooldown`))
          (set `self.A2OnCooldown` false))))))

(event `Ability2`
  (bind _returnvalue (`self.K2_GetActorLocation`))
  (bind _returnvalue_2 (`GameplayStatics.GetPlayerController` 0))
  ;[1 1 1] Ability2
  ;;[1 1 1] DamageAndKnock
  (`|ExecutionSequence`
    (:`then_0`
      (bind _outhits (`KismetSystemLibrary.SphereTraceMulti` _returnvalue _returnvalue 200.0 "TraceTypeQuery1"))
      (`NiagaraFunctionLibrary.SpawnSystemAtLocation` "/Game/Blueprints/Player/Abilities/N_AOE.N_AOE" (+ (`self.K2_GetActorLocation`) (* (* (`self.GetActorUpVector`) 200.0) -1.0)))
      (for _array_element _outhits
        (bind _asbp_melee_enemy_parent (cast `/Game/Blueprints/Enemies/BP_EnemyParent` (`.HitActor` (`GameplayStatics.BreakHitResult` _array_element))))
        (bind _damageoutput (`self.F_AbilityDamageSet` 2))
        (`GameplayStatics.ApplyDamage` _asbp_melee_enemy_parent _damageoutput null self)
        (bind (_returnvalue_x _returnvalue_y) (`KismetMathLibrary.BreakVector` (* (* (`self.GetActorForwardVector` _asbp_melee_enemy_parent) 1000.0) -1.0)))
        (`self.LaunchCharacter` _asbp_melee_enemy_parent (`KismetMathLibrary.MakeVector` _returnvalue_x _returnvalue_y 300.0) true true))
      (`/Game/Blueprints/HUD/WBP_MainHud.Ability2Used` (`self.MainWidgetRef`) (`KismetMathLibrary.FTrunc` (`self.Ability2Cooldown`))))
    (:`then_1`
      (`KismetSystemLibrary.Delay` 0.2)
      (`self.EnableInput` _returnvalue_2 _returnvalue_2)
      (set `self.A2OnCooldown` true)
      (`KismetSystemLibrary.Delay` (`self.Ability2Cooldown`))
      (set `self.A2OnCooldown` false))))

(fn `UserConstructionScript`
  (`parent.UserConstructionScript`))