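; Ranged player character with a looping bow attack and two cooldown abilities previewed on press and fired on release.
; Draw and release montages chain while left mouse is held, with events toggling the arrow mesh and spawning BP_Arrow.
; ArrowHit damages the closest target in range rather than a passed actor.
; Ability one box-traces boosted damage through melee enemies; ability two slows nearby ones and launches the player backward.
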(event `self.ReceiveBeginPlay`
  (`parent.ReceiveBeginPlay`)
  (`SkinnedMeshComponent.HideBoneByName` (`self.Mesh`) "Arrow" "PBO_None"))

(event `/Game/Blueprints/Player/BPI_PlayerInterface.Attack`
  (bind _mesh (`self.Mesh`))
  ;[1 1 1] BowAnim
  (`/Engine/EditorBlueprintResources/StandardMacros.DoOnce` false :!label _label
    (:`Completed`
      (set `self.Aiming` true)
      (`|PlayMontage` _mesh "/Game/Blueprints/Player/Ranged_Mesh/AttackAnims/AM_BowDraw.AM_BowDraw" :!label _label_2
        (:`OnBlendOut`
          (`|PlayMontage` _mesh "/Game/Blueprints/Player/Ranged_Mesh/AttackAnims/AM_BowRelase.AM_BowRelase"
            (:`OnBlendOut`
              (if (`PlayerController.IsInputKeyDown` (`GameplayStatics.GetPlayerController` 0) "LeftMouseButton")
                (goto _label_2)
                (else
                  (`self.ComboReset`))))))))))

(event `self.ComboReset`
  ;[1 1 1] BowAnim
  (set `self.Aiming` false)
  (goto _label :!via `Reset`))

(event `GrabbedArrow`
  ;[1 1 1] Hide/SpawnArrow
  (`SceneComponent.SetVisibility` (`self.ArrowMesh`) true false))

(event `SpawnArrow`
  (bind _capsulecomponent (`self.CapsuleComponent`))
  (bind _returnvalue_location (`KismetMathLibrary.BreakTransform` (`SceneComponent.K2_GetComponentToWorld` (`self.ArrowMesh`))))
  (bind _returnvalue (`SceneComponent.K2_GetComponentLocation` _capsulecomponent))
  ;[1 1 1] Hide/SpawnArrow
  (`SceneComponent.SetVisibility` (`self.ArrowMesh`) false false)
  (if (not (`self.InAbility1`))
    (`|SpawnActorFromClass` "/Game/Blueprints/Player/NewPlayers/BP_Arrow.BP_Arrow_C" (`KismetMathLibrary.MakeTransform` _returnvalue_location (`KismetMathLibrary.FindLookAtRotation` _returnvalue (+ _returnvalue (* (`SceneComponent.GetForwardVector` _capsulecomponent) 500.0))) (2.0 2.0 2.0)) "Undefined" "OverrideRootScale" null null)))

(event `ArrowHit`
  (params (Arrow :type "Actor Object Reference"))
  (bind _closest (`self.FindClosestTarget` (`self.TargetsInRange`)))
  (`GameplayStatics.ApplyDamage` _closest (`self.PlayerDamage`) null self))

(event `/Game/Blueprints/Player/BPI_PlayerInterface.A1-Pressed`
  ;[1 1 1] Aility1
  ;;[1 1 1] InitialPress
  (if (not (`self.A1OnCooldown`))
    (`SceneComponent.SetVisibility` (`self.Ability1Display`) true false)
    (set `self.RMB_Held?` false)))

(event `/Game/Blueprints/Player/BPI_PlayerInterface.A1-Released`
  (bind _returnvalue (`GameplayStatics.GetPlayerController` 0))
  (bind _mesh (`self.Mesh`))
  ;[1 1 1] Aility1
  ;;[1 1 1] InitialPress
  (if (`self.RMB_Held?`)
    _
    (elif (`SceneComponent.bVisible` (`self.Ability1Display`))
      (`SceneComponent.SetVisibility` (`self.Ability1Display`) false false)
      (set `self.InAbility1` true)
      (`|PlayMontage` _mesh "/Game/Blueprints/Player/Ranged_Mesh/AttackAnims/AM_BowDraw.AM_BowDraw" 1.5
        (:`then`
          (`self.DisableInput` _returnvalue _returnvalue))
        (:`OnBlendOut`
          (`|PlayMontage` _mesh "/Game/Blueprints/Player/Ranged_Mesh/AttackAnims/AM_BowRelase.AM_BowRelase" 1.5
            (:`OnBlendOut`
              (`self.ComboReset`)
              (`self.Ability1`))))))))

(event `self.Ability1`
  (bind _returnvalue (`GameplayStatics.GetPlayerController` 0))
  (bind _returnvalue_2 (`self.K2_GetActorLocation`))
  ;[1 1 1] Aility1
  ;;[1 1 1] AbilitySpawned
  (`|ExecutionSequence`
    (:`then_0`
      (bind _outhits (`KismetSystemLibrary.BoxTraceMulti` _returnvalue_2 (+ _returnvalue_2 (* (`self.GetActorForwardVector`) 900.0)) (50.0 50.0 50.0) (struct) "TraceTypeQuery1"))
      (`self.M_SpawnArrow`)
      (for _array_element _outhits
        (bind _asbp_melee_enemy_parent (cast `/Game/Blueprints/Enemies/BP_MeleeEnemyParent` (`.HitActor` (`GameplayStatics.BreakHitResult` _array_element))))
        (`GameplayStatics.ApplyDamage` _asbp_melee_enemy_parent (* (`self.PlayerDamage`) 1.8) null self))
      (`/Game/Blueprints/HUD/WBP_MainHud.Ability1Used` (`self.MainWidgetRef`) (`KismetMathLibrary.FTrunc` (`self.Ability1Cooldown`)))
      (set `self.InAbility1` false))
    (:`then_1`
      (`KismetSystemLibrary.Delay` 0.2)
      (`self.EnableInput` _returnvalue _returnvalue)
      (set `self.A1OnCooldown` true)
      (`KismetSystemLibrary.Delay` (`self.Ability1Cooldown`))
      (set `self.A1OnCooldown` false))))

(event `/Game/Blueprints/Player/BPI_PlayerInterface.A2-Pressed`
  ;[1 1 1] Ability2
  ;;[1 1 1] AbilityPressed
  (if (not (`self.A2OnCooldown`))
    (`SceneComponent.SetVisibility` (`self.Ability2Display`) true false)
    (set `self.RMB_Held?` false)))

(event `/Game/Blueprints/Player/BPI_PlayerInterface.A2-Released`
  ;[1 1 1] Ability2
  ;;[1 1 1] AbilityPressed
  (if (`self.RMB_Held?`)
    _
    (elif (`SceneComponent.bVisible` (`self.Ability2Display`))
      (`SceneComponent.SetVisibility` (`self.Ability2Display`) false false)
      (`self.ComboReset`)
      (`self.Ability2`))))

(event `self.Ability2`
  (bind _returnvalue (`self.K2_GetActorLocation`))
  (bind (_returnvalue_x _returnvalue_y) (`KismetMathLibrary.BreakVector` (`self.K2_GetActorLocation`)))
  (bind _ability2cooldown (`self.Ability2Cooldown`))
  ;[1 1 1] Ability2
  ;;[1 1 1] Ability 2 Dash
  (`|ExecutionSequence`
    (:`then_0`
      (`NiagaraFunctionLibrary.SpawnSystemAtLocation` "/Game/Blueprints/Player/Abilities/N_ShadowSphere.N_ShadowSphere" (`KismetMathLibrary.MakeVector` _returnvalue_x _returnvalue_y -100.0) (struct) (10.0 10.0 10.0))
      (bind _outhits (`KismetSystemLibrary.SphereTraceMulti` _returnvalue _returnvalue 200.0 "TraceTypeQuery1"))
      (for _array_element _outhits
        (bind _asbp_melee_enemy_parent (cast `/Game/Blueprints/Enemies/BP_MeleeEnemyParent` (`.HitActor` (`GameplayStatics.BreakHitResult` _array_element))))
        (`/Game/Blueprints/Enemies/BP_MeleeEnemyParent.Slowed` _asbp_melee_enemy_parent 50.0 5.0))
      (`self.LaunchCharacter` (0.0 0.0 250.0) false true)
      (`KismetSystemLibrary.Delay` 0.1)
      (`self.LaunchCharacter` (* (`self.GetActorForwardVector`) -3000.0) true true)
      (`/Game/Blueprints/HUD/WBP_MainHud.Ability2Used` (`self.MainWidgetRef`) (`KismetMathLibrary.FTrunc` _ability2cooldown)))
    (:`then_1`
      (set `self.A2OnCooldown` true)
      (`KismetSystemLibrary.Delay` _ability2cooldown)
      (set `self.A2OnCooldown` false))))

(fn `UserConstructionScript`
  (`parent.UserConstructionScript`))