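; BP_HealthPot is a health potion pickup item, a child Blueprint that overrides the PickedUp event.
; On pickup it casts the player pawn to BP_CharacterParent and calls FPotionPickedUp with type Health and an amount equal to a percentage of the character's max health.
; It then runs the parent PickedUp logic, which is skipped if the cast fails.
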(event `self.PickedUp`
  (bind _asbp_character_parent (cast `/Game/Blueprints/Player/NewPlayers/BP_CharacterParent` (`GameplayStatics.GetPlayerPawn` 0)))
  (`/Game/Blueprints/Player/NewPlayers/BP_CharacterParent.F_PotionPickedUp` _asbp_character_parent "Health" (* (/ (`/Game/Blueprints/Player/NewPlayers/BP_CharacterParent.Stat_MaxHealth` _asbp_character_parent) 100.0) 30.0))
  (`parent.PickedUp`))

(fn `UserConstructionScript`
  (`parent.UserConstructionScript`))