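; Base Blueprint for collectible items that the player picks up by overlap, with gear stats such as cost, tier and socket.
; BeginPlay loads those stats from a data table row by Name, then enables the pickup range after a short delay.
; Pickup runs once, adding the item to the player's CollectedItems unless one shares its Name, then moving it below the world instead of destroying it.
; The GearBought call is unconnected.
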(event `self.ReceiveBeginPlay`
  (bind _pickuprange (`self.PickUpRange`))
  (bind _returnvalue (`|GetDataTableRow` (`self.DataTableRef`) (`self.Name`))
    (:`then`
      (bind (_socket _cost _damage _health _movementspeed _tier _material) (break `/Game/Blueprints/Items/F_ItemDataStruct` _returnvalue))
      (set `self.Socket` _socket)
      (set `self.Cost` _cost)
      (set `self.Damage` _damage)
      (set `self.Health` _health)
      (set `self.MovementSpeed` _movementspeed)
      (set `self.Tier` _tier)
      (set `self.Material` _material)
      (`PrimitiveComponent.SetCollisionEnabled` _pickuprange "NoCollision")
      (`KismetSystemLibrary.Delay` 1.0)
      (`PrimitiveComponent.SetCollisionEnabled` _pickuprange "QueryOnly"))
    (:`RowNotFound`
      (`KismetSystemLibrary.PrintString` "SeriousError"))))

(event `self.PickUpRange.OnComponentBeginOverlap`
  (params (OverlappedComponent :type "PrimitiveComponent Object Reference") (OtherActor :type "Actor Object Reference") (OtherComp :type "PrimitiveComponent Object Reference") (OtherBodyIndex :type Integer) (bFromSweep :type Boolean) (SweepResult :type "HitResult Structure (by ref)"))
  (if (== OtherActor (`GameplayStatics.GetPlayerPawn` 0))
    (`self.PickedUp`)))

(event `PickedUp`
  ;[1 1 1] ItemPickedUp
  (bind _asbp_player_character_parent (cast `/Game/Blueprints/Player/BP_PlayerCharacterParent` (`GameplayStatics.GetPlayerPawn` 0)))
  (`/Engine/EditorBlueprintResources/StandardMacros.DoOnce` false
    (:`Completed`
      (bind _collecteditems (`/Game/Blueprints/Player/BP_PlayerCharacterParent.CollectedItems` _asbp_player_character_parent))
      (bind _iteminarray_out (`self.CheckIfItemIsInArray_F` _collecteditems))
      (if (not _iteminarray_out)
        (`KismetArrayLibrary.Array_Add` _collecteditems self)
        (`self.K2_SetActorLocation` (0.0 0.0 -1500.0))))))

(fn `CheckIfItemIsInArray_F`
  (params (Array :type "Array of /Game/Blueprints/Items/BP_CollectibleParent Object Reference"))
  (returns (ItemInArray_Out :type Boolean))
  (locals (ItemInArray :type Boolean))
  (for _array_element Array
    (if (== (`/Game/Blueprints/Items/BP_CollectibleParent.Name` _array_element) (`self.Name`))
      (set `local.ItemInArray` true)))
  (if (`local.ItemInArray`)
    (return true)
    (else
      (return false))))

(fn `UserConstructionScript`)