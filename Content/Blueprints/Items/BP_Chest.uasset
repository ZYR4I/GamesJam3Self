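; Loot chest that opens once when a player damages it with no melee enemies inside its sphere, healing the player and dropping one item.
; Temporarily spawns item classes far below the level to read socket and tier, deriving the player's hat, boot, sword and belt tiers.
; Random loot comes from unowned items one tier above those.
; Timelines swing the lid open and toss the item in an arc, with a coin burst.
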(event `self.ReceiveBeginPlay`)

(event `self.ReceiveAnyDamage`
  (params (Damage :type "Float (single-precision)") (DamageType :type "DamageType Object Reference") (InstigatedBy :type "Controller Object Reference") (DamageCauser :type "Actor Object Reference"))
  (bind _returnvalue (`self.GetActorForwardVector`))
  (bind _playerref (`self.PlayerRef`))
  (bind _returnvalue_2 (`SceneComponent.K2_GetComponentLocation` (`self.SpawnLocation`)))
  (bind _returnvalue_3 (+ (+ _returnvalue_2 (0.0 0.0 60.0)) (* _returnvalue -100.0)))
  (bind _asbp_player_character_parent (cast `/Game/Blueprints/Player/BP_PlayerCharacterParent` DamageCauser))
  (set `self.PlayerRef` _asbp_player_character_parent)
  (if (not (> (`KismetArrayLibrary.Array_Length` (`PrimitiveComponent.GetOverlappingActors` (`self.Sphere`) "/Game/Blueprints/Enemies/BP_MeleeEnemyParent.BP_MeleeEnemyParent_C")) 0))
    (`/Engine/EditorBlueprintResources/StandardMacros.DoOnce` false
      (:`Completed`
        (set `self.PlayersItems` (`/Game/Blueprints/Player/BP_PlayerCharacterParent.CollectedItems` _playerref))
        (for _array_element (`/Game/Blueprints/Player/BP_PlayerCharacterParent.CollectedItemsRef` _playerref)
          (`KismetArrayLibrary.Array_RemoveItem` (`self.AllItems`) _array_element)
          (bind _returnvalue_4 (`|SpawnActorFromClass` _array_element (`KismetMathLibrary.MakeTransform` (0.0 0.0 -5000.0)) "Undefined" "OverrideRootScale" null null))
          (switch `name` (`/Game/Blueprints/Items/BP_CollectibleParent.Socket` _returnvalue_4)
            (:`HatSocket`
              (`self.SetPlayerTiers` _returnvalue_4 :!label _label)
              (`self.K2_DestroyActor` _returnvalue_4))
            (:`BootSocket`
              (goto _label :!via `execute2`))
            (:`SwordSocket`
              (goto _label :!via `execute3`))
            (:`HipsSocket`
              (goto _label :!via `execute4`))))
        (bind (_direction _chestopen) (`Timeline|ChestOpen`)
          (:`Update`
            (`SceneComponent.K2_SetRelativeRotation` (`self.Scene`) (`KismetMathLibrary.RLerp` (struct) (struct :`Pitch` -60.0) _chestopen) false false))
          (:`Finished`
            (for _array_element_2 (`self.AllItems`)
              (`self.FindPossibleSpawns` _array_element_2)
              (`KismetArrayLibrary.Array_Add` (`self.PossibleSpawns`) _array_element_2))
            (`self.Opened`)
            (`/Game/Blueprints/Player/BP_PlayerCharacterParent.AddHealth` (`self.PlayerRef`) 150.0)
            (`NiagaraFunctionLibrary.SpawnSystemAtLocation` "/Game/Blueprints/Items/FX_CoinBurst.FX_CoinBurst" (`SceneComponent.K2_GetComponentLocation` (`self.SpawnLocation`)))
            (bind _returnvalue_5 (`|SpawnActorFromClass` (`KismetArrayLibrary.Array_Random` (`self.PossibleSpawns`)) (`KismetMathLibrary.Conv_VectorToTransform` (`SceneComponent.K2_GetComponentLocation` (`self.SpawnLocation`))) "Undefined" "OverrideRootScale" null null))
            (bind (_direction_2 _chestopen_2) (`Timeline|Timeline_0`)
              (:`Update`
                (`self.K2_SetActorLocation` _returnvalue_5 (`KismetMathLibrary.VLerp` _returnvalue_2 _returnvalue_3 _chestopen_2) false false))
              (:`Finished`
                (bind (_direction_3 _chestopen_3) (`Timeline|Timeline_1`)
                  (:`Update`
                    (`self.K2_SetActorLocation` _returnvalue_5 (`KismetMathLibrary.VLerp` _returnvalue_3 (+ (* _returnvalue -200.0) _returnvalue_2) _chestopen_3) false false)))))))))))

(event `Opened`)

(fn `UserConstructionScript`)